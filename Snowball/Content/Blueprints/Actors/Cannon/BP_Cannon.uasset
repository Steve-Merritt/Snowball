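; BP_Cannon is a cannon actor that fires projectiles automatically and endlessly from BeginPlay.
; After each FireRate delay it spawns a BP_Projectile at ProjectileSpawnPoint, scaled by ProjectileScale, then plays the barrel timeline.
; The timeline drives the barrel's relative Y location, and its Cannon Fired event loops back to the delay to start the next shot.
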(event EventBeginPlay
  (Utilities|FlowControl|Delay (Variables|CannonProperties|GetFire%20Rate) :!label _label)
  (CallFunction|SpawnProjectile)
  (bind _barrel_location (Timeline|Cannon%20Barrel%20Animation PlayFromStart)
    (:Update
      (CallFunction|MoveCannonBarrel _barrel_location))
    (:Cannon%20Fired
      (goto _label))))

(fn ConstructionScript)

(fn SpawnProjectile
  (bind _projectile_spawn_point (Variables|Default|GetProjectile%20Spawn%20Point))
  (Game|SpawnActorfromClass "/Game/Blueprints/Actors/Projectiles/BP_Projectile.BP_Projectile_C" (Math|Transform|MakeTransform (Transformation|GetWorldLocation _projectile_spawn_point) (Transformation|GetWorldRotation _projectile_spawn_point) (Math|Conversions|ToVector(Float) (Variables|CannonProperties|GetProjectile%20Scale))) "AlwaysSpawn" 0 0))

(fn MoveCannonBarrel
  (params (Cannon%20Barrel%20Y%20Location :type Float%20%28single-precision%29))
  (Transformation|SetRelativeLocation (Variables|Default|GetCannon%20Barrel) (Math|Vector|MakeVector 0.0 Cannon%20Barrel%20Y%20Location 0.0) false false))