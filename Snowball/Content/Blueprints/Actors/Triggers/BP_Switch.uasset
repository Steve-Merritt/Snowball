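; BP_Switch is a one-way switch actor that activates a linked Triggerable when its pillar mesh registers a hit.
; The hit latches Activated, and Tick then calls Activate on the Triggerable once.
; Tick also feeds DoMove a frame-rate-scaled step, accumulating a clamped lerp alpha that slides the switch from its start location along its forward vector by SwitchOffset.
; Nothing in the graph resets it.
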(event OnComponentHit(SM_Fire_Fort_Pillar_1f)
  (params (HitComponent :type Primitive%20Component%20Object%20Reference) (OtherActor :type Actor%20Object%20Reference) (OtherComp :type Primitive%20Component%20Object%20Reference) (NormalImpulse :type Vector :default "0, 0, 0") (Hit :type Hit%20Result%20Structure%20%28by%20ref%29))
  (Variables|Default|SetActivated true))

(event EventBeginPlay
  (bind _self self)
  (bind _output_get (Variables|Default|SetStartLocation (Transformation|GetActorLocation _self)))
  (Variables|Default|SetEndLocation (+ _output_get (* (Transformation|GetActorForwardVector _self) (Variables|Default|GetSwitchOffset)))))

(event EventTick
  (params (DeltaSeconds :type Float%20%28single-precision%29))
  (Variables|Default|SetMoveSpeedThisFrame (* DeltaSeconds (Variables|Default|GetMoveSpeed)))
  (if (Variables|Default|GetActivated)
    (if (Variables|Default|GetTriggerable%20Activated)
      _
      (else
        (Default|Activate (Variables|Default|GetTriggerable))
        (Variables|Default|SetTriggerable%20Activated true)))
    (CallFunction|DoMove (Variables|Default|GetMoveSpeedThisFrame))))

(fn ConstructionScript)

(fn DoMove
  (params (MoveSpeed :type Float%20%28single-precision%29))
  (bind _output_get (Variables|Default|SetLerpAlpha (Math|Float|Clamp(Float) (+ MoveSpeed (Variables|Default|GetLerpAlpha)))))
  (Transformation|SetActorLocation (Math|Vector|Lerp(Vector) (Variables|Default|GetStartLocation) (Variables|Default|GetEndLocation) _output_get) false false))