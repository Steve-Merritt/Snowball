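; BP_Tooltip is a one-shot trigger actor that shows a tutorial-style message on the player pawn's HUD.
; Any overlap displays the configured Message at full opacity, optionally stopping the player and highlighting the healthbar.
; When the overlap ends, a FadeOut timeline fades the text and border, then hides any highlight and destroys the actor.
; Both events act on player pawn 0 without checking which actor overlapped.
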(event Collision|EventActorBeginOverlap
  (params (OtherActor :type Actor%20Object%20Reference))
  (bind _asbp_player_pawn (Utilities|Casting|CastToBP_PlayerPawn (Game|Player|GetPlayerPawn 0)))
  (if (Variables|Default|GetShouldStopPlayer)
    (Default|StopPlayer _asbp_player_pawn))
  (Rendering|Components|TextRender|SetText (Variables|/Game/UI/HUD.HUD_C|GetDialogMessage (Variables|/Game/Blueprints/Pawns/BP_PlayerPawn.BP_PlayerPawn_C|GetHUD%20Reference _asbp_player_pawn)) (Variables|Default|GetMessage))
  (Class|TextBlock|SetOpacity (Variables|/Game/UI/HUD.HUD_C|GetDialogMessage (Variables|/Game/Blueprints/Pawns/BP_PlayerPawn.BP_PlayerPawn_C|GetHUD%20Reference _asbp_player_pawn)) 1.0)
  (Widget|SetRenderOpacity (Variables|/Game/UI/HUD.HUD_C|GetDialogMessageBorder (Variables|/Game/Blueprints/Pawns/BP_PlayerPawn.BP_PlayerPawn_C|GetHUD%20Reference _asbp_player_pawn)) 1.0)
  (if (Variables|Default|GetHighlight%20Healthbar)
    (Widget|SetVisibility (Variables|/Game/UI/HUD.HUD_C|GetHealthbarHighlight (Variables|/Game/Blueprints/Pawns/BP_PlayerPawn.BP_PlayerPawn_C|GetHUD%20Reference _asbp_player_pawn)) "Visible")))

(event Collision|EventActorEndOverlap
  (params (OtherActor :type Actor%20Object%20Reference))
  (bind _asbp_player_pawn (Utilities|Casting|CastToBP_PlayerPawn (Game|Player|GetPlayerPawn 0)))
  (bind _opacity (Timeline|FadeOut Play)
    (:Update
      (Class|TextBlock|SetOpacity (Variables|/Game/UI/HUD.HUD_C|GetDialogMessage (Variables|/Game/Blueprints/Pawns/BP_PlayerPawn.BP_PlayerPawn_C|GetHUD%20Reference _asbp_player_pawn)) _opacity)
      (Widget|SetRenderOpacity (Variables|/Game/UI/HUD.HUD_C|GetDialogMessageBorder (Variables|/Game/Blueprints/Pawns/BP_PlayerPawn.BP_PlayerPawn_C|GetHUD%20Reference _asbp_player_pawn)) _opacity))
    (:Finished
      (if (Variables|Default|GetHighlight%20Healthbar)
        (Widget|SetVisibility (Variables|/Game/UI/HUD.HUD_C|GetHealthbarHighlight (Variables|/Game/Blueprints/Pawns/BP_PlayerPawn.BP_PlayerPawn_C|GetHUD%20Reference (stale Collision|EventActorBeginOverlap _asbp_player_pawn))) "Hidden"))
      (Actor|DestroyActor))))

(fn ConstructionScript)