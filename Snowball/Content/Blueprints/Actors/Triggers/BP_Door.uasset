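; BP_Door is a trigger-activated door actor that swings open 90 degrees in yaw once unlocked.
; BeginPlay stores the starting rotation and derives the open rotation from it.
; Activate sets the Unlocked flag, and Tick then advances a clamped alpha by RotationSpeed times delta time and lerps the actor rotation toward open.
; It has no logic to close or relock.
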(event EventBeginPlay
  (bind _output_get (Variables|Default|SetStartRotation (Transformation|GetActorRotation)))
  (Variables|Default|SetEndRotation (Math|Rotator|CombineRotators _output_get (Math|Rotator|MakeRotator 0.0 0.0 9e+01))))

(event EventActivate
  (Variables|Default|SetUnlocked true))

(event EventTick
  (params (DeltaSeconds :type Float%20%28single-precision%29))
  (bind _output_get (Variables|Default|SetRotationSpeedThisFrame (* DeltaSeconds (Variables|Default|GetRotationSpeed))))
  (if (Variables|Default|GetUnlocked)
    (bind _output_get_2 (Variables|Default|SetRotationAlpha (Math|Float|Clamp(Float) (+ _output_get (Variables|Default|GetRotationAlpha)))))
    (Transformation|SetActorRotation (Math|Rotator|Lerp(Rotator) (Variables|Default|GetStartRotation) (Variables|Default|GetEndRotation) _output_get_2))))

(fn ConstructionScript)