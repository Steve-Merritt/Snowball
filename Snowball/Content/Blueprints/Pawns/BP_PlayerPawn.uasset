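; Player pawn for a rolling physics ball that melts over time, with input axes applying torque to its sphere.
; Each tick drains health at the melt rate, which climbs to a capped multiple of its base below the lava heat height, and updates the HUD bar.
; Empty health or hitting a Lava physical surface triggers death, which fades out and reloads the current level through a DoOnce gate.
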(event OnComponentHit(Sphere)
  (params (HitComponent :type Primitive%20Component%20Object%20Reference) (OtherActor :type Actor%20Object%20Reference) (OtherComp :type Primitive%20Component%20Object%20Reference) (NormalImpulse :type Vector :default "0, 0, 0") (Hit :type Hit%20Result%20Structure%20%28by%20ref%29))
  (switch Utilities|FlowControl|Switch|SwitchonEPhysicalSurface (Collision|GetSurfaceType Hit)
    (:SurfaceType1
      (Physics|SetPhysicsLinearVelocity (Variables|Default|GetSphere) "0, 0, 0" false "None")
      (CallFunction|EventDeath))))

(event Custom|Event%20Death
  (Utilities|RestartLevel))

(event EventBeginPlay
  (Variables|Melting|SetMeltRate (Variables|Melting|GetBaseMeltRate))
  (bind _returnvalue (UserInterface|CreateWidget "/Game/UI/HUD.HUD_C"))
  (bind _output_get (Variables|Default|SetHUD%20Reference _returnvalue))
  (UserInterface|Viewport|AddtoViewport _output_get 0)
  (CameraFades|StartCameraFade :self (Game|GetPlayerCameraManager 0) :FromAlpha 1.0 :Duration 2.0))

(event EventTick
  (params (DeltaSeconds :type Float%20%28single-precision%29))
  (bind _lavaheatheight (Variables|Default|GetLavaHeatHeight))
  (Variables|Default|SetDeltaSeconds DeltaSeconds)
  (if (< (.z (Transformation|GetActorLocation self)) (Variables|Default|GetLavaHeatHeight))
    (bind _output_get (Variables|Default|SetUnitLavaHeat (/ (- _lavaheatheight 1.0) _lavaheatheight)))
    (Variables|Melting|SetMeltRate (Math|Float|Clamp(Float) (* (Variables|Melting|GetMeltRate) (+ _output_get 1.0)) 0.0 (* (Variables|Melting|GetBaseMeltRate) (Variables|Melting|GetMaxMeltRateScale))))
    (else
      (Variables|Melting|SetMeltRate (Variables|Melting|GetBaseMeltRate))))
  (CallFunction|SetHealth))

(event Input|AxisEvents|InputAxisUnitMoveFwd
  (params (AxisValue :type Float%20%28single-precision%29))
  (Class|PrimitiveComponent|AddTorqueinRadians (Variables|Default|GetSphere) (Math|Vector|MakeVector 0.0 (* AxisValue (Variables|Default|GetTorque)) 0.0) "None" true))

(event Input|AxisEvents|InputAxisUnitMoveLateral
  (params (AxisValue :type Float%20%28single-precision%29))
  (Class|PrimitiveComponent|AddTorqueinRadians (Variables|Default|GetSphere) (Math|Vector|MakeVector (* AxisValue (Variables|Default|GetTorque)) 0.0 0.0) "None" true))

(fn ConstructionScript)

(fn SetHealth
  (bind _output_get (Variables|Default|SetUnitHealth (Math|Float|Clamp(Float) (- (Variables|Default|GetUnitHealth) (* (Variables|Default|GetDeltaSeconds) (Variables|Melting|GetMeltRate))))))
  (Progress|SetPercent (Variables|/Game/UI/HUD.HUD_C|GetHealthBar (Variables|Default|GetHUD%20Reference)) _output_get)
  (if (== _output_get 0.0)
    (CallFunction|EventDeath)))